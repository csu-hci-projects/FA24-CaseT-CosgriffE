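; BP_MovingHazard is a hazard actor that moves back and forth and damages the player.
; Tick offsets it without sweep along the normalized Direction at Speed, while a looping timer reverses Direction every TimeToChange seconds.
; Any overlap subtracts Damage from the first-person character's Health and calls CheckHealth, or opens Level2 if Health is already at or below zero.
; The overlap always targets player 0, whichever actor triggered it.
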(event Custom|ChangeDirection
  ;[1 1 1] Moving Target
  (Variables|Default|SetDirection (* (Variables|Default|GetDirection) -1.0)))

(event EventTick
  (params (DeltaSeconds :type Float%20%28single-precision%29))
  ;[1 1 1] Moving Target
  (Transformation|AddActorWorldOffset (* (Math|Vector|Normalize (Variables|Default|GetDirection)) (* (Variables|Default|GetSpeed) (Utilities|Time|GetWorldDeltaSeconds)))))

(event EventBeginPlay
  ;[1 1 1] Moving Target
  (Utilities|Time|SetTimerbyEvent (delegate Custom|ChangeDirection) (Variables|Default|GetTimeToChange) true))

(event Collision|EventActorBeginOverlap
  (params (OtherActor :type Actor%20Object%20Reference))
  ;[1 1 1] Decreasing Health and Restarting
  (bind _asbp_first_person_character (Utilities|Casting|CastToBP_FirstPersonCharacter (Game|GetPlayerCharacter 0)))
  (if (<= (Variables|/Game/FirstPerson/Blueprints/BP_FirstPersonCharacter.BP_FirstPersonCharacter_C|GetHealth _asbp_first_person_character) 0)
    (Game|OpenLevel(byObjectReference) "/Game/MyLevels/Level-2.Level-2")
    (else
      (Variables|/Game/FirstPerson/Blueprints/BP_FirstPersonCharacter.BP_FirstPersonCharacter_C|SetHealth _asbp_first_person_character (- (Variables|/Game/FirstPerson/Blueprints/BP_FirstPersonCharacter.BP_FirstPersonCharacter_C|GetHealth _asbp_first_person_character) (Variables|Default|GetDamage)))
      (Default|CheckHealth _asbp_first_person_character))))

(fn ConstructionScript)